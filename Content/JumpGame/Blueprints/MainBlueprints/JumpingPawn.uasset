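; Player pawn for a touch-controlled hold-to-charge platform-hopping game, handling jumping, scoring, audio and death.
; Holding touch builds charge and squashes the pawn; release launches it toward the next stage at charge-scaled speed.
; A first landing gets graded by the stage, doubling consecutive high scores, spawning a random stage along +X or +Y and arming any bonus timer.
; A zero grade triggers a physics tumble off the edge, while dispatchers broadcast state changes.
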(event `self.ReceiveBeginPlay`
  (add `self.TouchStageOrNewStageEvents` (delegate `SomeHitCausedUpdateEvent`))
  (add `self.normalScoreGain` (delegate `playNormalScoreAudio`))
  (add `self.doubleScoreGain` (delegate `playHighScoreAuidio`)))

(event `SomeHitCausedUpdateEvent`
  (`self.DestroyTimerForAdditionalGrade`))

(event `playNormalScoreAudio`
  (`AudioComponent.Play` (`self.normalScore`) 0.0))

(event `playHighScoreAuidio` :!signature `self.doubleScoreGain`
  (params (grade :type Integer) (location :type "Vector Structure"))
  (`AudioComponent.Play` (`self.highScore`) 0.0))

(event `Key|Touch1`
  (params (Key :type "Key Structure"))
  ;[1 1 1] 输入处理
  (:`Pressed`
    (`self.EnableTouchInput` :!label _label ; 检查角色是否死亡，死亡状态不会执行接下来的任何一步
      (:`canPress`
        (`self.StartCharingWork`))
      (:`canRelease`
        ;;[1 1 1] 蓄力结束，并跳跃，此时设置不允许蓄力（直到落到下一个平台才能进行下一次蓄力）
        (if (`self.canDoJump`)
          (set `self.canDoJump` false)
          (set `self.isCharging` false)
          (`self.StartJumpingWork`)
          (`self.jumpStart`)))))
  (:`Released`
    (goto _label :!via `release`)))

(event `self.ReceiveTick`
  (params (DeltaSeconds :type "Float (single-precision)"))
  (`self.UpdatePerTick` DeltaSeconds) ; 每帧执行的更新函数
  ;[1 1 1] 死亡时判断角色高度
  (if (`self.isDead`)
    (`/Engine/EditorBlueprintResources/StandardMacros.DoOnce` false
      (:`Completed`
        (`self.CheckHeightDispatch`) ; 物体一旦被标记为死亡状态，就要每一帧去检查它，使得关卡蓝图能够在某个时间得到这个消息
      ))
    (else
      ;[1 1 1] 空中时判断角色高度
      (if (not (`self.canDoJump`))
        (`self.CheckHeightDispatch`)))))

(event `self.ReceiveHit`
  (params (MyComp :type "PrimitiveComponent Object Reference") (Other :type "Actor Object Reference") (OtherComp :type "PrimitiveComponent Object Reference") (bSelfMoved :type Boolean) (HitLocation :type "Vector Structure") (HitNormal :type "Vector Structure") (NormalImpulse :type "Vector Structure") (Hit :type "HitResult Structure (by ref)"))
  ;[1 1 1] 碰撞事件发生
  (bind _asstage (cast `/Game/JumpGame/Blueprints/Stages/Stage` Other))
  (set `self.currentStage` _asstage)
  (`self.TouchStageOrNewStageEvents`) ; 通知撞击平台事件
  (set `self.canDoJump` true) ; 可以开始下一次蓄力了
  (`self.HItStageProcess` HitLocation ; 撞击的平台的逻辑处理，包括得分等判断，只有在第一次撞击的时候才执行后面的代码
    (:`isFirstHit`
      (`self.FirstHitOnStage` HitLocation))))

(fn `AddGrade`
  (params (additionalGrade :type Integer))
  (set `self.gainedScore` (+ additionalGrade (`self.gainedScore`))))

(fn `AimJumpDirection`
  (bind _returnvalue (* (`self.nextStageLocation`) (1.0 1.0 0.0)))
  (bind _returnvalue_2 (* (`self.K2_GetActorLocation`) (1.0 1.0 0.0)))
  (bind _output_get (set `self.movingDirection` (`KismetMathLibrary.GetDirectionUnitVector` _returnvalue_2 _returnvalue))) ; 更新跳跃方向
  (set `MovementComponent.Velocity` (* _output_get (* (`self.chargingPower`) (`self.SCALE_MOVE_SPEED`))) (`self.CharacterMovement`)) ; 设置速度
  ;[1 1 1] 修正棋子的转向，朝着新平台翻转
  (`SceneComponent.K2_SetRelativeRotation` (`self.Mesh`) (`KismetMathLibrary.FindLookAtRotation` _returnvalue_2 _returnvalue) false false) ; 修改带有动画的网格的旋转方向，让它对准跳跃的方向旋转
)

(fn `AnalysisScore`
  (params (grade :type Integer) (isFirstHit :type Boolean) (DropDirection :type Integer) (hitLocation :type "Vector Structure"))
  (locals (currentScore :type Integer))
  (bind _returnvalue (and (>= (`self.lastScore`) 2) (>= (`local.currentScore`) 2)))
  (bind _output_get (set `local.currentScore` grade))
  (`self.FallOnLowScore` _output_get isFirstHit DropDirection)
  (if (and isFirstHit (not (`self.isDead`)))
    ;[1 1 1] 更新LastScore，在这个函数中，LastScore存储的就是现在这一次的得分情况
    (set `self.lastScore` (`KismetMathLibrary.SelectInt` (* (`self.lastScore`) 2) (`local.currentScore`) _returnvalue))
    ;[1 1 1] 判断是普通得分还是累积高分
    (if _returnvalue
      (`self.doubleScoreGain` (`self.lastScore`) hitLocation)
      (else
        (`self.normalScoreGain`)))
    (`self.AddGrade` (`self.lastScore`)) ; 更新分数，注意这个函数中LastScore存储的是本次的得分
    (return)))

(fn `CreateRandomShapeStage`
  (params (InitLocation :type "Vector Structure"))
  (returns (returnStage :type "/Game/JumpGame/Blueprints/Stages/Stage Object Reference"))
  (locals (storeReturnStage :type "/Game/JumpGame/Blueprints/Stages/Stage Object Reference") (newStageTransform :type "Transform Structure") (NUM_MAX_STAGE_TYPES :type Integer :default 7))
  (set `local.newStageTransform` (`KismetMathLibrary.MakeTransform` InitLocation))
  (switch `int` (`KismetMathLibrary.RandomIntegerInRange` 0 (- (`local.NUM_MAX_STAGE_TYPES`) 1))
    (:`0`
      (bind _returnvalue (`|SpawnActorFromClass` "/Game/JumpGame/Blueprints/Stages/normalStage1.normalStage1_C" (`local.newStageTransform`) "Undefined" "OverrideRootScale" null null))
      (set `local.storeReturnStage` _returnvalue))
    (:`1`
      (bind _returnvalue_2 (`|SpawnActorFromClass` "/Game/JumpGame/Blueprints/Stages/normalStage2.normalStage2_C" (`local.newStageTransform`) "Undefined" "OverrideRootScale" null null))
      (set `local.storeReturnStage` _returnvalue_2))
    (:`2`
      (bind _returnvalue_3 (`|SpawnActorFromClass` "/Game/JumpGame/Blueprints/Stages/normalStage5.normalStage5_C" (`local.newStageTransform`) "Undefined" "OverrideRootScale" null null))
      (set `local.storeReturnStage` _returnvalue_3))
    (:`3`
      (bind _returnvalue_4 (`|SpawnActorFromClass` "/Game/JumpGame/Blueprints/Stages/normalStage6.normalStage6_C" (`local.newStageTransform`) "Undefined" "OverrideRootScale" null null))
      (set `local.storeReturnStage` _returnvalue_4))
    (:`4`
      (bind _returnvalue_5 (`|SpawnActorFromClass` "/Game/JumpGame/Blueprints/Stages/superMarketStage.superMarketStage_C" (`local.newStageTransform`) "Undefined" "OverrideRootScale" null null)) ; 超市平台
      (set `local.storeReturnStage` _returnvalue_5))
    (:`5`
      (bind _returnvalue_6 (`|SpawnActorFromClass` "/Game/JumpGame/Blueprints/Stages/musicStage.musicStage_C" (`local.newStageTransform`) "Undefined" "OverrideRootScale" null null)) ; 音乐台
      (set `local.storeReturnStage` _returnvalue_6))
    (:`6`
      (bind _returnvalue_7 (`|SpawnActorFromClass` "/Game/JumpGame/Blueprints/Stages/magicStage.magicStage_C" (`local.newStageTransform`) "Undefined" "OverrideRootScale" null null)) ; 魔方平台
      (set `local.storeReturnStage` _returnvalue_7)))
  (return (`local.storeReturnStage`)))

(fn `DestroyTimerForAdditionalGrade`
  (`/Engine/EditorBlueprintResources/StandardMacros.IsValid` (`self.timerHandlerForAdditionalGrade`)
    (:`Is Valid`
      (`/Game/JumpGame/Blueprints/Stages/Stage.DestroyTimerForAdditionalGrade` (`self.timerHandlerForAdditionalGrade`)))))

(fn `DoTheDeathJob`
  (params (theDirectionIndex :type Integer))
  (locals (direction :type Integer))
  (bind _capsulecomponent (`self.CapsuleComponent`))
  (if (not (`self.doneDeathJob`))
    (set `self.doneDeathJob` true) ; 没有的话才执行接下来的代码
    (set `local.direction` theDirectionIndex)
    (`AudioComponent.Play` (`self.deadAudio`) 0.0)
    (`self.StopAllAudioExceptDead`) ; 终止其他声效播放
    (`self.DestroyTimerForAdditionalGrade`)
    ;[1 1 1] 棋子的各种状态标志
    (set `self.isDead` true) ; 手动将棋子标记为死亡状态
    (set `self.isCharging` false)
    (set `self.canDoJump` false)
    ;[1 1 1] 设置布娃娃状态
    (`Controller.SetIgnoreMoveInput` (`GameplayStatics.GetPlayerController` 0) true)
    (`PrimitiveComponent.SetSimulatePhysics` _capsulecomponent true)
    (`PrimitiveComponent.SetPhysicsMaxAngularVelocityInDegrees` _capsulecomponent 10.0 false "None")
    (`PrimitiveComponent.SetLinearDamping` _capsulecomponent 1.0)
    (`PrimitiveComponent.SetAngularDamping` _capsulecomponent 1000.0)
    (`PrimitiveComponent.SetMassOverrideInKg` _capsulecomponent "None" 100.0 true)
    (`PrimitiveComponent.SetCollisionResponseToChannel` _capsulecomponent "ECC_PhysicsBody" "ECR_Overlap")
    ;[1 1 1] 当棋子掉落在平台的某个边缘的时候，把它往外面推，线性速度置空，给它一点角速度，让它翻转掉落
    (bind _velocity (`self.GenerateFallLinearVelocity` (`local.direction`)))
    (`PrimitiveComponent.SetPhysicsLinearVelocity` (`self.CapsuleComponent`) _velocity false "None")
    (bind _returnangularvelocity (`self.GenerateFallAngularVelocity` (`local.direction`)))
    (`PrimitiveComponent.SetPhysicsAngularVelocityInDegrees` (`self.CapsuleComponent`) _returnangularvelocity false "None")
    (`ActorComponent.Deactivate` (`self.chargingParticle`))))

(fn `DropAnotherStage`
  (bind _location (`self.UpdateNextStageLocation`)) ; 更新下一个平台的坐标
  (`self.CreateRandomShapeStage` _location) ; 随机创建平台并且初始化
)

(fn `FallOnLowScore`
  (params (score :type Integer) (isFirstScore :type Boolean) (DropDirection :type Integer))
  (if (== score 0)
    (`self.DoTheDeathJob` DropDirection) ; 分数为0表示角色掉出了平台范围
  ))

(fn `FirstHitOnStage`
  (params (hitLocation :type "Vector Structure"))
  (if (not (`self.isDead`))
    (if (not (`/Game/JumpGame/Blueprints/Stages/Stage.StartedStage` (`self.currentStage`)))
      (`GameplayStatics.SpawnEmitterAtLocation` "/Game/JumpGame/Particles/hitParticle.hitParticle" hitLocation) ; 生成撞击的烟尘效果
    )
    (`self.DropAnotherStage`) ; 新平台生成
    (`self.TouchStageOrNewStageEvents`) ; 如果生成了一个新平台，这里就再调用一次撞击事件调度器
    ;[1 1 1] 看看现在撞击的这个平台有没有额外的分数可以拿
    (bind _haveadditionalgrade (`/Game/JumpGame/Blueprints/Stages/Stage.IsHaveAdditionalGrade` (`self.currentStage`)))
    (if _haveadditionalgrade
      (bind _timerhandler (`/Game/JumpGame/Blueprints/Stages/Stage.PawnAskForAdditionalGrade` (`self.currentStage`) self))
      (`self.DestroyTimerForAdditionalGrade`)
      (set `self.timerHandlerForAdditionalGrade` _timerhandler))))

(fn `GenerateFallAngularVelocity`
  (params (Direction :type Integer))
  (returns (returnAngularVelocity :type "Vector Structure"))
  (locals (angularVelocity :type "Vector Structure") (singleVelocityStrength :type "Float (double-precision)" :default 5.0))
  (bind _singlevelocitystrength (`local.singleVelocityStrength`))
  (bind _returnvalue (* (`local.singleVelocityStrength`) -1.0))
  (switch `int` Direction
    (:`0`
      ;[1 1 1] 选择设置
      (set `local.angularVelocity` (0.0 0.0 0.0)))
    (:`1`
      (set `local.angularVelocity` (`KismetMathLibrary.MakeVector` 0.0 _singlevelocitystrength)))
    (:`2`
      (set `local.angularVelocity` (`KismetMathLibrary.MakeVector` 0.0 _returnvalue)))
    (:`3`
      (set `local.angularVelocity` (`KismetMathLibrary.MakeVector` _returnvalue)))
    (:`4`
      (set `local.angularVelocity` (`KismetMathLibrary.MakeVector` _singlevelocitystrength))))
  (return (`local.angularVelocity`)))

(fn `GenerateFallLinearVelocity`
  (params (direction :type Integer))
  (returns (velocity :type "Vector Structure"))
  (locals (linearVelocity :type "Vector Structure") (SingleVelocityStrength :type "Float (double-precision)" :default 10.0))
  (bind _singlevelocitystrength (`local.SingleVelocityStrength`))
  (bind _returnvalue (* (`local.SingleVelocityStrength`) -1.0))
  (switch `int` direction
    (:`0`
      ;[1 1 1] 选择设置
      (set `local.linearVelocity` (0.0 0.0 0.0)))
    (:`1`
      (set `local.linearVelocity` (`KismetMathLibrary.MakeVector` _singlevelocitystrength)))
    (:`2`
      (set `local.linearVelocity` (`KismetMathLibrary.MakeVector` _returnvalue)))
    (:`3`
      (set `local.linearVelocity` (`KismetMathLibrary.MakeVector` 0.0 _singlevelocitystrength)))
    (:`4`
      (set `local.linearVelocity` (`KismetMathLibrary.MakeVector` 0.0 _returnvalue))))
  (return (`local.linearVelocity`)))

(fn `SetEnableScaleHeight`
  (params (enable :type Boolean))
  (bind _output_get (set `self.enableScaleHeight` enable))
  (if _output_get
    _
    (else
      _))
  (`self.SetScaleHeight` 1.0))

(fn `SetScaleHeight`
  (params (scaleHeight :type "Float (double-precision)"))
  (bind _output_get (set `self.currentScaleHeight` scaleHeight))
  (`self.K2_SetActorTransform` (`KismetMathLibrary.MakeTransform` (`self.K2_GetActorLocation`) (`self.K2_GetActorRotation`) (`KismetMathLibrary.MakeVector` 1.0 1.0 _output_get))))

(fn `StartCharingWork`
  ;[1 1 1] 蓄力开始，重置蓄力值
  (set `self.isCharging` true)
  (set `self.chargingPower` 0.0)
  (`AudioComponent.Play` (`self.chargingAudio`) 0.0) ; 播放蓄力音效
  (`self.charingStart`) ; 事件通知
  ;[1 1 1] 播放粒子的集中效果
  (`ActorComponent.Activate` (`self.chargingParticle`) false)
  (`self.SetEnableScaleHeight` true) ; 蓄力开始，棋子开始缩放形体
)

(fn `StartJumpingWork`
  ;[1 1 1] 音效设置
  (`AudioComponent.Stop` (`self.chargingAudio`))
  (`AudioComponent.Play` (`self.jumpAudio`) 0.0)
  (`self.AimJumpDirection`) ; 瞄准新平台的方向
  ;[1 1 1] 翻滚动画播放
  (`SkeletalMeshComponent.PlayAnimation` (`self.Mesh`) "/Game/JumpGame/MeshesOrAnimation/jumpingPawn/AnimationPawn_anima.AnimationPawn_anima" false)
  (`SkeletalMeshComponent.SetPlayRate` (`self.Mesh`) (`self.AnimationRate`))
  (`self.Jump`) ; 执行跳跃操作
  (`ActorComponent.Deactivate` (`self.chargingParticle`))
  (`self.SetEnableScaleHeight` false) ; 关闭棋子之前的蓄力形变
)

(fn `StopAllAudioExceptDead`
  (`AudioComponent.Stop` (`self.chargingAudio`))
  (`AudioComponent.Stop` (`self.jumpAudio`)))

(fn `UpdateHeightScale`
  (params (deltaTime :type "Float (double-precision)"))
  (if (`self.enableScaleHeight`)
    (`self.SetScaleHeight` (`KismetMathLibrary.FMax` (- (`self.currentScaleHeight`) (* deltaTime (`self.SCALE_SPEED_PER_SECOND`))) (`self.MIN_SCALE_PAWN`)))))

(fn `UpdateNextStageLocation`
  (returns (location :type "Vector Structure"))
  (bind _default_next_stage_height (`self.DEFAULT_NEXT_STAGE_HEIGHT`))
  (bind _returnvalue (`KismetMathLibrary.RandomFloatInRange` 200.0 (`self.MAX_NEXT_STAGE_DIST`)))
  (bind _x (.x (`self.prevStageLocation`)))
  (bind _y (.y (`self.prevStageLocation`)))
  ;[1 1 1] 更新prevStageLocation和nextStageLocation并返回数据
  (set `self.prevStageLocation` (`self.nextStageLocation`))
  (bind _output_get (set `self.nextStageLocation` (`KismetMathLibrary.SelectVector` (`KismetMathLibrary.MakeVector` (+ _returnvalue _x) _y _default_next_stage_height) (`KismetMathLibrary.MakeVector` _x (+ _y _returnvalue) _default_next_stage_height) (`KismetMathLibrary.RandomBoolFromStream` (`self.randomStreamForLeftOrRight`)))))
  (return _output_get))

(fn `UpdatePerTick`
  (params (DeltaSeconds :type "Float (double-precision)"))
  (locals (scaleCharingAudioVolumen :type "Float (double-precision)" :default 0.2) (deltaTime :type "Float (double-precision)"))
  (set `local.deltaTime` DeltaSeconds)
  (if (`self.isCharging`)
    ;[1 1 1] 检查当前状态是否处于蓄力中，如果是的话，根据每帧的时间长度增加ChargingPower
    (bind _output_get (set `self.chargingPower` (+ (`self.chargingPower`) (* (`local.deltaTime`) (`self.CHARGED_POWER_PER_SECOND`)))))
    ;[1 1 1] 逐渐提高充能的声音
    (`AudioComponent.SetVolumeMultiplier` (`self.chargingAudio`) (* _output_get (`local.scaleCharingAudioVolumen`)))
    ;[1 1 1] 更新棋子形变
    (`self.UpdateHeightScale` (`local.deltaTime`))))

(fn `UserConstructionScript`
  (bind _charactermovement (`self.CharacterMovement`))
  ;[1 1 1] 初始化PrevStageLocation和NextStageLocation置，默认为当前的这个JumpingPawn对象的坐标
  (bind _output_get (set `self.prevStageLocation` (.location (`self.GetTransform`))))
  (set `self.nextStageLocation` _output_get)
  (set `self.randomStreamForLeftOrRight` (`KismetMathLibrary.MakeRandomStream` 0))
  ;[1 1 1] 计算并设置AnimationRate，根据跳跃初速度、重力缩放值以及一个Scale属性进行计算
  (set `self.AnimationRate` (* (/ (`CharacterMovementComponent.GravityScale` _charactermovement) (/ (`CharacterMovementComponent.JumpZVelocity` _charactermovement) 1000.0)) (`self.SCALE_JUMP_ANIMATION_RATE`))))