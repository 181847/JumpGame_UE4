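; Camera actor for the jump game that glides horizontally toward the midpoint between the previous and next stages.
; UpdateStageLocations stores both stage positions, and UpdateCenterLocation sets their average as the target, enabling movement if it changed.
; Tick steps by a fixed Speed per frame, not scaled by delta time, along the XY part of the direction.
; Movement stops only when the full 3D location, Z included, nearly equals the target.
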(event `self.ReceiveTick`
  (params (DeltaSeconds :type "Float (single-precision)"))
  (bind _returnvalue (`self.K2_GetActorLocation`))
  (if (`self.isNeedMoving`)
    (`self.K2_SetActorLocation` (+ (* (* (`KismetMathLibrary.GetDirectionUnitVector` _returnvalue (`self.targetLocation`)) (`self.speed`)) (1.0 1.0 0.0)) _returnvalue))
    ;[1 1 1] 如果到达指定的位置，则停止移动
    (if (== _returnvalue (`self.targetLocation`))
      (set `self.isNeedMoving` false))))

(fn `UpdateCenterLocation`
  (bind _returnvalue (* (+ (`self.prevStageLocation`) (`self.nextStageLocation`)) 0.5))
  (if (!= _returnvalue (`self.targetLocation`))
    (set `self.targetLocation` _returnvalue)
    (set `self.isNeedMoving` true)))

(fn `UpdateStageLocations`
  (params (prevLocation :type "Vector Structure") (nextLocation :type "Vector Structure"))
  (set `self.prevStageLocation` prevLocation)
  (set `self.nextStageLocation` nextLocation)
  (`self.UpdateCenterLocation`))

(fn `UserConstructionScript`)