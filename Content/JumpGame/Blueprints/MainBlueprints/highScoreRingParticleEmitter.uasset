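; Short-lived actor in the jump game that plays a series of high-score ring particles at its own location.
; InitAndShow runs once, clamping the score to a maximum and spawning the first ring immediately, then repeating on a looping timer.
; Each ring halves the remaining score, so ring count grows logarithmically with score.
; Once the score drops to one or below, it clears the timer and destroys itself.
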(fn `InitAndShow`
  (params (scoreToShow :type Integer))
  (`/Engine/EditorBlueprintResources/StandardMacros.DoOnce` false ; 只能{初始化}和{开始发射粒子}一次
    (:`Completed`
      (set `self.scoreToShow` (`KismetMathLibrary.Min` scoreToShow (`self.CLAMP_MAX_SCORE`)))
      (set `self.emitLocation` (`self.K2_GetActorLocation`))
      (`self.Show`))))

(fn `NewParticle`
  (if (> (`self.scoreToShow`) 1)
    ;[1 1 1] 还有分数环没有被显示完
    (set `self.scoreToShow` (/ (`self.scoreToShow`) 2)) ; 更新分数
    (`GameplayStatics.SpawnEmitterAtLocation` "/Game/JumpGame/Particles/highScoreParticle.highScoreParticle" (`self.emitLocation`)) ; 生成圆环粒子
    (else
      ;[1 1 1] 当分数小于等于1的时候，就删除{计时器}和{自己}
      (`KismetSystemLibrary.K2_ClearAndInvalidateTimerHandle` (`self.timeHandler`))
      (`self.K2_DestroyActor`))))

(fn `Show`
  (`self.NewParticle`) ; 第一次立即创建一个粒子
  (`KismetSystemLibrary.K2_SetTimer` self "NewParticle" (`self.TIME_BETWEEN_TWO_RING`) true))

(fn `UserConstructionScript`)