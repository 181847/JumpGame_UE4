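; Base Blueprint for a cylinder stage in the jump game, with support for an additional grade award.
; Its construction script runs the parent's, then calls Init with variables for shape, radius, bonus grade and the wait before that bonus.
; The AdditionalGradeGiven event only prints a debug string; BeginPlay, overlap and Tick are disabled placeholders.
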(event `self.AdditionalGradeGiven`
  (`KismetSystemLibrary.PrintString` "cylingder extra grade gained" true true (struct :`G` 0.073006 :`B` 1.0 :`A` 1.0)))

(fn `UserConstructionScript`
  (`parent.UserConstructionScript`)
  (`self.Init` (`self.DERVIED_IS_SQUARE`) (`self.DERVIED_RADIUS`) (`self.ADDITIONAL_GRADE`) (`self.WAITING_TIME_ADDITIONAL_GRADE`)))