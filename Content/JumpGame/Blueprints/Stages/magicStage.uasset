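; Magic stage Blueprint for the jump game, a platform variant that can award an additional score and animates when it does.
; Its construction script passes its own shape, radius, bonus score and waiting time to the inherited Init.
; The AdditionalGradeGiven event plays the stage animation once on AnimationMesh at a set play rate, so the animation runs only when the bonus is earned.
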(event `self.AdditionalGradeGiven`
  (`SkeletalMeshComponent.PlayAnimation` (`self.animationMesh`) "/Game/JumpGame/MeshesOrAnimation/stage3Animation/AnimationStage3_Anim.AnimationStage3_Anim" false)
  (`SkeletalMeshComponent.SetPlayRate` (`self.animationMesh`) (`self.ANIMATION_PLAY_RATE`)))

(fn `UserConstructionScript`
  (`parent.UserConstructionScript`)
  (`self.Init` (`self.DERVIED_IS_SQUARE`) (`self.DERVIED_RADIUS`) (`self.ADDITIONAL_GRADE`) (`self.WAITING_TIME_ADDITIONAL_GRADE`)))