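; Supermarket stage for the jump game, a child stage Blueprint that configures an inherited stage base with its own shape and bonus-grade settings.
; The construction script calls Init with the square flag, radius, additional grade and waiting time for that grade.
; When the AdditionalGradeGiven event fires, it plays AnimationMesh once, without looping, at a set play rate.
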(event `self.AdditionalGradeGiven`
  (`SkeletalMeshComponent.Play` (`self.animationMesh`) false)
  (`SkeletalMeshComponent.SetPlayRate` (`self.animationMesh`) (`self.ANIMATION_PLAY_RATE`)))

(fn `UserConstructionScript`
  (`parent.UserConstructionScript`)
  (`self.Init` (`self.DERVIED_IS_SQUARE`) (`self.DERVIED_RADIUS`) (`self.ADDITIONAL_GRADE`) (`self.WAITING_TIME_ADDITIONAL_GRADE`)))